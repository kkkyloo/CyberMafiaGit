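; Construction-script wire prop that lays spline mesh segments along an editable spline, with selectable wire variants and thickness.
; SplineMeshVar chooses segments between spline points or at fixed Spacing along the length with scaled direction tangents.
; WireVar picks the mesh component and whether it has one or two material slots.
; Dynamic MI_Wire instances receive colors, dirt tint, specular, roughness and a TextureVar-selected texture set.
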(fn ConstructionScript
  (|Wire))