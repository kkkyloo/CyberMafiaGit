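; Base enemy character driven by AIC_Enemy_Base, with patrol route, movement speed presets, weapons and animation overlay states.
; Picked-up weapons go through ACWeapon and attach as a child actor on hand_r, which receives fire messages.
; GetCamera supplies randomly offset aim points near the AI's attack target.
; Player hits report damage on the first BP_Enemy_Base found and decrement Hp; at zero the enemy ragdolls and notifies its controller.
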(event Custom|FootSteps
  (Audio|PlaySoundatLocation "/Game/Sounds/MovementSound/MS_Footstep.MS_Footstep" (Transformation|GetActorLocation) "0, 0, 0" 1.0 1.0 0.0 0 0 0 0))

(event Custom|CalculateDirection
  ;[1 1 1] Calc Dir
  (Variables|Movement|SetDirection (Class|KismetAnimationLibrary|CalculateDirection (Transformation|GetVelocity) (Transformation|GetActorRotation))))

(event Custom|OverlayToIdle
  ;[1 1 1] Overlay State
  (CallFunction|SetOverlay (Variables|Overlays|GetOverlayIdle)))

(event Custom|Set%20Overlay
  (params (OverlayState :type EN_OverlaysStates%20Enum :default "NewEnumerator0"))
  ;[1 1 1] Overlay State
  (Variables|Overlays|SetOverlay%20State OverlayState))

(event Custom|Fire%20Off
  ;[1 1 1] Fireing
  (Variables|WeaponSystem|SetFireing false)
  (Class|BPIWeapon|FireOff(Message) (Variables|/Script/Engine.ChildActorComponent|GetChildActor (Variables|Default|GetHandObject))))

(event Custom|Fire%20On
  (bind _handobject (Variables|Default|GetHandObject))
  (bind _childactor (Variables|/Script/Engine.ChildActorComponent|GetChildActor _handobject))
  ;[1 1 1] Fireing
  (if (Variables|Default|GetCanDoSomthing)
    (Variables|WeaponSystem|SetFireing true)
    (Class|BPIWeapon|Fireon(Message) _childactor self)
    (Utilities|FlowControl|Delay 1.0)
    (Class|BPIWeapon|FireOff(Message) _childactor)))

(event EventBeginPlay
  ;[0.05098 0.05098 0.05098] Link
  (bind _asabp_manny (Utilities|Casting|CastToABP_Manny (Components|SkeletalMesh|GetAnimInstance (Variables|Character|GetMesh))))
  (Variables|Default|SetLinkToABPManny _asabp_manny))

(event Game|Damage|EventAnyDamage
  (params (Damage :type Float%20%28single-precision%29) (DamageType :type Damage%20Type%20Object%20Reference) (InstigatedBy :type Controller%20Object%20Reference) (DamageCauser :type Actor%20Object%20Reference))
  (bind _hp (Variables|Default|GetHp))
  (if (== DamageCauser (Game|GetPlayerCharacter 0))
    (bind _returnvalue (Actor|GetActorOfClass "BP_Enemy_Base_C"))
    ;[1 1 1] Damage
    (Class|AISenseDamage|ReportDamageEvent _returnvalue 0 0.0 "0, 0, 0" "0, 0, 0" "None")
    (Math|Integer|DecrementInt _hp
      (:%20%20
        (if (<= _hp 0)
          (Physics|SetSimulatePhysics (Variables|Character|GetMesh) true)
          (Variables|Default|SetCanDoSomthing false)
          (bind _asaic_enemy_base (Utilities|Casting|CastToAIC_Enemy_Base (Pawn|GetController)))
          (Default|Dead _asaic_enemy_base)
          (Collision|SetCollisionEnabled (Variables|Collision|GetCapsuleComponent) "NoCollision"))))))

(event EventTick
  (params (DeltaSeconds :type Float%20%28single-precision%29)))

(fn ConstructionScript)

(fn AttachtoHand
  (params (Overlay%20Idle :type EN_OverlaysStates%20Enum :default "NewEnumerator0") (Actor%20BP :type Actor%20Soft%20Class%20Reference) (Socket%20Transform :type Transform))
  (Variables|Overlays|SetOverlayIdle Overlay%20Idle)
  (if (Utilities|IsValidSoftClassReference Actor%20BP)
    (bind _returnvalue (Utilities|LoadClassAssetBlocking Actor%20BP))
    (bind _asactor (Utilities|Casting|CastToActorClass _returnvalue))
    (ChildActorComponent|SetChildActorClass (Variables|Default|GetHandObject) _asactor)
    (Transformation|AttachComponentToComponent (Variables|Default|GetHandObject) (Variables|Character|GetMesh) "hand_r" "SnapToTarget" "SnapToTarget" "SnapToTarget" true)
    (Transformation|SetRelativeTransform (Variables|Default|GetHandObject) Socket%20Transform true true)
    (else
      (ChildActorComponent|SetChildActorClass (Variables|Default|GetHandObject) 0)))
  (CallFunction|SetOverlay (Variables|Overlays|GetOverlayIdle))
  (Variables|Default|SetHaveGun true)
  (return))

(fn GetCamera
  (bind _asaic_enemy_base (Utilities|Casting|CastToAIC_Enemy_Base (AI|GetAIController self)))
  (return (Transformation|GetSocketLocation (Variables|Character|GetMesh) "head") (Math|Vector|MakeVector (Math|Random|RandomFloatinRange (.x (Transformation|GetActorLocation (Variables|/Game/Blueprints/Enemy/AI/AIC_Enemy_Base.AIC_Enemy_Base_C|GetAttackTarget _asaic_enemy_base))) (+ (.x (Transformation|GetActorLocation (Variables|/Game/Blueprints/Enemy/AI/AIC_Enemy_Base.AIC_Enemy_Base_C|GetAttackTarget _asaic_enemy_base))) 5e+01)) (Math|Random|RandomFloatinRange (.y (Transformation|GetActorLocation (Variables|/Game/Blueprints/Enemy/AI/AIC_Enemy_Base.AIC_Enemy_Base_C|GetAttackTarget _asaic_enemy_base))) (+ (.y (Transformation|GetActorLocation (Variables|/Game/Blueprints/Enemy/AI/AIC_Enemy_Base.AIC_Enemy_Base_C|GetAttackTarget _asaic_enemy_base))) 5e+01)) (Math|Random|RandomFloatinRange (.z (Transformation|GetActorLocation (Variables|/Game/Blueprints/Enemy/AI/AIC_Enemy_Base.AIC_Enemy_Base_C|GetAttackTarget _asaic_enemy_base))) (+ (.z (Transformation|GetActorLocation (Variables|/Game/Blueprints/Enemy/AI/AIC_Enemy_Base.AIC_Enemy_Base_C|GetAttackTarget _asaic_enemy_base))) 5e+01))) true))

(fn GetPatrol
  (return (Variables|Default|GetPatrolRoute)))

(fn GetWeaponName
  (return (Variables|/Game/Blueprints/WeaponSystem/Inventory/Categories/Weapons/AC_Weapon.AC_Weapon_C|GetActiveWeapon (Variables|Default|GetAC_Weapon))))

(fn PickUpWeapon
  (params (WeaponName :type Name :default "None"))
  (Default|Give (Variables|Default|GetAC_Weapon) WeaponName)
  (bind _value (Default|CycleUp (Variables|Default|GetAC_Weapon)))
  (CallFunction|AttachtoHand (.OverlayIdle (Utilities|Struct|BreakS_Weapon _value)) (.Actor_BP (Utilities|Struct|BreakS_Weapon _value)) (.SocketTransform (Utilities|Struct|BreakS_Weapon _value)))
  (Variables|Overlays|SetOverlayScope (.OverlyScope (Utilities|Struct|BreakS_Weapon _value)))
  (Variables|Overlays|SetOverlayIdle (.OverlayIdle (Utilities|Struct|BreakS_Weapon _value)))
  (Variables|Overlays|SetOverlayRun (.OverlayRun (Utilities|Struct|BreakS_Weapon _value)))
  (return true))

(fn SetMovementSpeed
  (params (Speed :type E_MovementSpeed%20Enum :default "NewEnumerator0"))
  (bind _output_get (Variables|/Script/Engine.CharacterMovementComponent|SetMaxWalkSpeed (Variables|Character|GetCharacterMovement) (Utilities|Select :Index Speed :NewEnumerator0 0.0 :NewEnumerator1 3e+02 :NewEnumerator2 6e+02 :NewEnumerator3 2e+02)))
  (return _output_get))