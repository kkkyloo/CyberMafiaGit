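; Key interactive object that shows a widget and enables the player's CanTake flag when its Sre component is overlapped.
; The overlap does not check which actor entered, and the key destroys itself 2.1 seconds later without waiting for input.
; Ending the overlap hides the widget but leaves CanTake set.
; A separate Destroy event removes the actor immediately.
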(event OnComponentBeginOverlap(sre)
  (params (OverlappedComponent :type Primitive%20Component%20Object%20Reference) (OtherActor :type Actor%20Object%20Reference) (OtherComp :type Primitive%20Component%20Object%20Reference) (OtherBodyIndex :type Integer) (bFromSweep :type Boolean) (SweepResult :type Hit%20Result%20Structure%20%28by%20ref%29))
  (Rendering|SetVisibility (Variables|Default|GetWidget) true false)
  (bind _asbp_player (Utilities|Casting|CastToBP_Player (Game|GetPlayerCharacter 0)))
  (Variables|/Game/Blueprints/Player/BP_Player.BP_Player_C|SetCanTake _asbp_player true)
  (Utilities|FlowControl|Delay 2.1)
  (Actor|DestroyActor))

(event OnComponentEndOverlap(sre)
  (params (OverlappedComponent :type Primitive%20Component%20Object%20Reference) (OtherActor :type Actor%20Object%20Reference) (OtherComp :type Primitive%20Component%20Object%20Reference) (OtherBodyIndex :type Integer))
  (Rendering|SetVisibility (Variables|Default|GetWidget) false false))

(event Custom|Destroy
  (Actor|DestroyActor))

(fn ConstructionScript)