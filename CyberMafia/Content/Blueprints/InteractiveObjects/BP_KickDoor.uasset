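; Interactive door that the player character kicks open, triggered once when something begins overlapping its box.
; It disables player input, slides the player along world X to a skeletal mesh's position, then plays a kick montage while a timeline yaws the Sphere component open.
; A flag-guarded, delayed sequence in that timeline's update plays the door sound, removes collision, emits noise at the door and restores player control.
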(event OnComponentBeginOverlap(Box)
  (params (OverlappedComponent :type Primitive%20Component%20Object%20Reference) (OtherActor :type Actor%20Object%20Reference) (OtherComp :type Primitive%20Component%20Object%20Reference) (OtherBodyIndex :type Integer) (bFromSweep :type Boolean) (SweepResult :type Hit%20Result%20Structure%20%28by%20ref%29))
  (Utilities|FlowControl|DoOnce false
    (:Completed
      (bind _asbp_player (Utilities|Casting|CastToBP_Player (Game|GetPlayerCharacter 0)))
      (Input|DisableInput _asbp_player 0)
      (Default|DefaultState _asbp_player)
      (bind _alpha (Timeline|Timeline Play)
        (:Update
          (Transformation|SetActorTransform _asbp_player (Math|Transform|MakeTransform (Math|Vector|MakeVector (Math|Float|Lerp (.x (.location (Transformation|GetActorTransform _asbp_player))) (.x (.location (Transformation|GetWorldTransform (Variables|Default|GetSkelewetalMesh)))) _alpha) (.y (.location (Transformation|GetActorTransform _asbp_player))) (.z (.location (Transformation|GetActorTransform _asbp_player)))) (.rotation (Transformation|GetActorTransform _asbp_player)) (.scale (Transformation|GetActorTransform _asbp_player)))))
        (:Finished
          (Animation|PlayAnimMontage _asbp_player "/Game/Animation/Characters/Mannequins/Animations/Quinn/MyAnimation/Door/MmaKick_UE_Montage.MmaKick_UE_Montage" 1.0 "None")
          (bind _kickdoor (Timeline|OpenDoor Play)
            (:Update
              (Transformation|SetRelativeRotation (Variables|Default|GetSphere) (Math|Rotator|MakeRotator 0.0 0.0 (Math|Float|Lerp 0.0 -1.2e+02 _kickdoor)) false false)
              (if (not (Variables|Default|GetSound))
                (Utilities|FlowControl|Delay 0.6)
                (Audio|SpawnSoundatLocation "/Game/Sounds/door-open.door-open" (Transformation|GetWorldLocation (Variables|Default|GetDoor)) "0, 0, 0" 1.0 1.0 0.0 0 0)
                (Variables|Default|SetSound true)
                (Collision|SetCollisionEnabled (Variables|Default|GetDoor) "NoCollision")
                (Utilities|FlowControl|Delay 0.4)
                (Class|Actor|MakeNoise 1.0 (Game|GetPlayerCharacter 0) (Transformation|GetWorldLocation (Variables|Default|GetSphere)) 0.0 "None")
                (Default|OverlaytoIdle _asbp_player)
                (Default|MoveEnable _asbp_player)
                (Input|EnableInput _asbp_player 0)))))))))

(event OnComponentEndOverlap(Box)
  (params (OverlappedComponent :type Primitive%20Component%20Object%20Reference) (OtherActor :type Actor%20Object%20Reference) (OtherComp :type Primitive%20Component%20Object%20Reference) (OtherBodyIndex :type Integer)))

(event Input|ActionEvents|InputActionInteract
  (params (Key :type Key%20Structure)))

(fn ConstructionScript)